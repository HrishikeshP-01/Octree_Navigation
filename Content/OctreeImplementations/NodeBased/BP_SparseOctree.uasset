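; Sparse octree navigation test actor that builds a node graph and finds a path between two chosen nodes.
; The construction script generates the octree recursively or by level from MaxSide at the origin, using MinSide as a size setting, then derives the graph.
; It redraws debug views of the graph, path and start node's neighbors.
; Event graph is unused and occupancy visualization is disconnected.
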(event EventBeginPlay)

(event Collision|EventActorBeginOverlap
  (params (OtherActor :type Actor%20Object%20Reference)))

(event EventTick
  (params (DeltaSeconds :type Float%20%28single-precision%29)))

(fn ConstructionScript
  (bind _maxside (Variables|Default|GetmaxSide))
  (bind _graphnodes (Variables|Default|GetgraphNodes))
  (bind _startnode (Variables|Default|GetStartNode))
  (bind _output (Utilities|Array|Get(acopy) _graphnodes _startnode))
  (Class|ASparseOctree|SetVariables 0 0 0.0 _maxside (Variables|Default|GetminSide))
  (Class|ASparseOctree|GenerateOctree _maxside "0, 0, 0")
  (Class|ASparseOctree|GenerateGraph)
  (Rendering|Debug|FlushPersistentDebugLines)
  (Class|ASparseOctree|VisualizeGraph)
  (Class|ASparseOctree|FindPathBetweenNodes _output (Utilities|Array|Get(acopy) _graphnodes (Variables|Default|GetEndNode)))
  (Class|ASparseOctree|VisualizePath)
  (Class|ASparseOctree|VisualizeNeighborNodes _output))